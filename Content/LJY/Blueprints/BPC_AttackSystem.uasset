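; Attack component for BP_TopDownCharacter that runs a four-step greatsword combo and sword hit detection.
; IA_Attack plays the montage for the current combo counter; a montage notify unlocks and advances the next step, while a timer resets the counter.
; StartSwordTrace starts a looping timer that line-traces between the sword's top and bottom points, calling ApplyDamage on "Damageable" actors behind a delayed DoOnce gate.
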(event `Start Sword Trace`
  ; Sword Trace
  (`KismetSystemLibrary.K2_SetTimerDelegate` (delegate `Sword Trace Loop`) 10.0 true true 0.0 1.0))

(event `StopSwordTrace`
  ; Sword Trace
  (`KismetSystemLibrary.K2_ClearAndInvalidateTimerHandle` (`self.SwordTraceLoop`)))

(event `Sword Trace Loop`
  (bind _as_bp_top_down_character (`self.As BP Top Down Character`))
  ; Sword Trace
  (bind (_outhit _returnvalue) (`KismetSystemLibrary.LineTraceSingle` (`SceneComponent.K2_GetComponentLocation` (`/Game/TopDown/Blueprints/BP_TopDownCharacter.SwordTopPoint` _as_bp_top_down_character)) (`SceneComponent.K2_GetComponentLocation` (`/Game/TopDown/Blueprints/BP_TopDownCharacter.SwordBottomPoint` _as_bp_top_down_character)) "TraceTypeQuery1"))
  ; Damage
  (if _returnvalue
    (bind (_bblockinghit _binitialoverlap _time _distance _location _impactpoint _normal _impactnormal _physmat _hitactor) (`GameplayStatics.BreakHitResult` _outhit))
    (if (`Actor.ActorHasTag` _hitactor "Damageable")
      (`/Engine/EditorBlueprintResources/StandardMacros.DoOnce` false :!label _label
        (:`Completed`
          (bind _returnvalue_2 (`GameplayStatics.ApplyDamage` _hitactor))
          (`KismetSystemLibrary.PrintString` (`KismetStringLibrary.Conv_DoubleToString` _returnvalue_2))
          (`KismetSystemLibrary.Delay` 1.0)
          (goto _label :!via `Reset`))))))

(event `self.ReceiveBeginPlay`
  (bind _asbp_top_down_character (cast `/Game/TopDown/Blueprints/BP_TopDownCharacter` (`self.GetOwner`)))
  (bind _output_get (set `self.As BP Top Down Character` _asbp_top_down_character))
  (set `self.Character Mesh` (`Character.Mesh` _output_get)))

(event `EnhancedInput|/Game/LJY/Input/IA_Attack`
  (params (ActionValue :type Boolean) (ElapsedSeconds :type "Float (double-precision)") (TriggeredSeconds :type "Float (double-precision)") (InputAction :type "InputAction Object Reference" :default "/Game/LJY/Input/IA_Attack.IA_Attack"))
  (bind _character_mesh (`self.Character Mesh`))
  (:`Triggered`
    (if (not (`self.is Attack`))
      (`/Engine/EditorBlueprintResources/StandardMacros.DoOnce` false :!label _label_2
        (:`Completed`
          (set `self.is Attack` true)
          (switch `int` (`self.Combo Counter`)
            (:`0`
              (`|PlayMontage` _character_mesh "/Game/LJY/Animation/Great_Sword_Pack/slashMontage/great_sword_slash_Montage.great_sword_slash_Montage"
                (:`then`
                  (`KismetSystemLibrary.K2_SetTimerDelegate` (delegate `ResetCounter`) 1.0 :!label _label_3)
                  (goto _label_2 :!via `Reset`))
                (:`OnNotifyBegin`
                  (set `self.is Attack` false)
                  (set `self.Combo Counter` 1))))
            (:`1`
              (`|PlayMontage` _character_mesh "/Game/LJY/Animation/Great_Sword_Pack/slashMontage/great_sword_slash__3__Montage.great_sword_slash__3__Montage"
                (:`then`
                  (goto _label_3))
                (:`OnNotifyBegin`
                  (set `self.is Attack` false)
                  (set `self.Combo Counter` 2))))
            (:`2`
              (`|PlayMontage` _character_mesh "/Game/LJY/Animation/Great_Sword_Pack/slashMontage/great_sword_slash__4__Montage.great_sword_slash__4__Montage"
                (:`then`
                  (goto _label_3))
                (:`OnNotifyBegin`
                  (set `self.is Attack` false)
                  (set `self.Combo Counter` 3))))
            (:`3`
              (`|PlayMontage` _character_mesh "/Game/LJY/Animation/Great_Sword_Pack/slashMontage/great_sword_slash__5__Montage.great_sword_slash__5__Montage"
                (:`then`
                  (goto _label_3))
                (:`OnNotifyBegin`
                  (set `self.is Attack` false)
                  (set `self.Combo Counter` 0))))))))))

(event `ResetCounter`
  (set `self.Combo Counter` 0))