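; Test actor Blueprint that turns to face player character 0 and chases it while something overlaps its Sphere component.
; Sphere begin and end overlaps switch Speed on and off, without checking which actor triggered them.
; Tick always rotates toward the player, passing the same direction as X and Z to MakeRotFromXZ, and moves along it by Speed and delta time without sweep.
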(event `self.Sphere.OnComponentEndOverlap`
  (params (OverlappedComponent :type "PrimitiveComponent Object Reference") (OtherActor :type "Actor Object Reference") (OtherComp :type "PrimitiveComponent Object Reference") (OtherBodyIndex :type Integer))
  (set `self.Speed` 0.0))

(event `self.Sphere.OnComponentBeginOverlap`
  (params (OverlappedComponent :type "PrimitiveComponent Object Reference") (OtherActor :type "Actor Object Reference") (OtherComp :type "PrimitiveComponent Object Reference") (OtherBodyIndex :type Integer) (bFromSweep :type Boolean) (SweepResult :type "HitResult Structure (by ref)"))
  (set `self.Speed` 100.0))

(event `self.ReceiveTick`
  (params (DeltaSeconds :type "Float (single-precision)"))
  (bind _output_get (set `self.Direction` (`KismetMathLibrary.Normal` (- (`self.K2_GetActorLocation` (`GameplayStatics.GetPlayerCharacter` 0)) (`self.K2_GetActorLocation`)))))
  (`self.K2_SetActorRotation` (`KismetMathLibrary.MakeRotFromXZ` _output_get _output_get))
  (`self.K2_SetActorLocation` (+ (`self.K2_GetActorLocation`) (* (`self.Speed`) (`self.Direction`) (`GameplayStatics.GetWorldDeltaSeconds`)))))

(fn `UserConstructionScript`)