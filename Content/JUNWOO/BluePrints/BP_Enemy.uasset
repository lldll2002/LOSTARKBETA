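; Boss enemy that chases and attacks the player through a gimmick phase; its death shows the success screen and quits the game.
; Overlap volumes set tracing/attack state; Tick moves it manually and handles phase changes.
; AnyDamage feeds BPCEnemyStatsystem: health, then a paralyzation gauge resolving into groggy or big attack, then post-gimmick health.
; Custom events toggle limb hitboxes, gated by resettable DoOnce, and a just-guard window that punishes failed guards.
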(event `self.ReceiveBeginPlay`
  ; 초기설정
  (bind _asabp_enemy_2 (cast `/Game/JUNWOO/enemy/ABP_Enemy_2` (`SkeletalMeshComponent.GetAnimInstance` (`self.Mesh`))))
  (set `self.As ABP Enemy 2` _asabp_enemy_2)
  (`Widget.SetVisibility` (`WidgetComponent.GetUserWidgetObject` (`self.Enemy_Widget`)) "Hidden"))

(event `self.tmp_detecter.OnComponentBeginOverlap`
  (params (OverlappedComponent :type "PrimitiveComponent Object Reference") (OtherActor :type "Actor Object Reference") (OtherComp :type "PrimitiveComponent Object Reference") (OtherBodyIndex :type Integer) (bFromSweep :type Boolean) (SweepResult :type "HitResult Structure (by ref)"))
  ; 공격, 추격 시스템
  ;; 추격 범위에 들어온다면 추격
  (set `self.speed` 300.0)
  (set `self.IsTracing` true))

(event `self.attack range.OnComponentEndOverlap`
  (params (OverlappedComponent :type "PrimitiveComponent Object Reference") (OtherActor :type "Actor Object Reference") (OtherComp :type "PrimitiveComponent Object Reference") (OtherBodyIndex :type Integer))
  (if (`self.GimmickState`)
    ; 공격, 추격 시스템
    ;; 공격 범위에 나간다면 다시 추격
    (set `self.speed` 300.0)
    (cast `/Game/TopDown/Blueprints/BP_TopDownCharacter` OtherActor)
    (set `self.IsAttack` false)
    (set `self.IsTracing` true)
    (else
      (set `self.speed` 0.0)
      (cast `/Game/TopDown/Blueprints/BP_TopDownCharacter` OtherActor)
      (set `self.IsAttack` false)
      (set `self.IsTracing` true))))

(event `self.attack range.OnComponentBeginOverlap`
  (params (OverlappedComponent :type "PrimitiveComponent Object Reference") (OtherActor :type "Actor Object Reference") (OtherComp :type "PrimitiveComponent Object Reference") (OtherBodyIndex :type Integer) (bFromSweep :type Boolean) (SweepResult :type "HitResult Structure (by ref)"))
  ; 공격, 추격 시스템
  ;; 공격 범위에 들어온다면 추격을 멈추고 공격
  (set `self.speed` 0.0)
  (cast `/Game/TopDown/Blueprints/BP_TopDownCharacter` OtherActor)
  (set `self.IsAttack` true)
  (set `self.IsTracing` false))

(event `self.tmp_detecter.OnComponentEndOverlap`
  (params (OverlappedComponent :type "PrimitiveComponent Object Reference") (OtherActor :type "Actor Object Reference") (OtherComp :type "PrimitiveComponent Object Reference") (OtherBodyIndex :type Integer))
  ; 공격, 추격 시스템
  ;; 추격 범위에서 나간다면 다시 대기 상태
  (cast `/Game/TopDown/Blueprints/BP_TopDownCharacter` OtherActor)
  (set `self.speed` 0.0)
  (set `self.IsTracing` false))

(event `self.ReceiveAnyDamage`
  (params (Damage :type "Float (single-precision)") (DamageType :type "DamageType Object Reference") (InstigatedBy :type "Controller Object Reference") (DamageCauser :type "Actor Object Reference"))
  (set `self.Damage Causer` DamageCauser)
  (bind (_up_vector _right_vector) (message `/Game/LJY/UI/BPI_Player.IF_GetVectors` (`GameplayStatics.GetPlayerPawn` 0)))
  (`|SpawnActorFromClass` "/Game/LJY/UI/BP_Damage.BP_Damage_C" (`KismetMathLibrary.MakeTransform` (+ (`SceneComponent.GetSocketLocation` (`self.Mesh`) "Start") (* _up_vector 20) (* _right_vector 20))) "Undefined" "MultiplyWithRoot" null Damage null)
  (if (`self.GimmickSwith`)
    (bind (_isgimmick _currenthealth) (`/Game/JUNWOO/components/BPC_enemy_statsystem.decrease health` (`self.BPC_enemy_statsystem`) Damage))
    (set `self.Is Gimmick` _isgimmick)
    (set `self.Current Health` _currenthealth)
    (elif (`self.GimmickSwitch2`)
      (bind (_currentpargauge _maxpargauge _gimmickswitch3) (`/Game/JUNWOO/components/BPC_enemy_statsystem.decrease paralyzation` (`self.BPC_enemy_statsystem`) Damage))
      (`self.UpdateHealthBar` _currentpargauge _maxpargauge)
      (if _gimmickswitch3
        (bind (_gimmickend _isgroggy _isbigattack) (`/Game/JUNWOO/components/BPC_enemy_statsystem.Gimmick` (`self.BPC_enemy_statsystem`) _currentpargauge))
        (`Widget.SetVisibility` (`WidgetComponent.GetUserWidgetObject` (`self.Enemy_Widget`)) "Hidden")
        (set `self.Gimmick End` _gimmickend)
        (set `self.IsGroggy` _isgroggy)
        (set `self.IsBigAttack` _isbigattack)
        (set `self.State` false)
        (elif (`self.JustGuard`)
          (set `self.JustGuard` false)
          (`KismetSystemLibrary.Delay` 2.0)
          (`self.PlayAnimMontage` "/Game/JUNWOO/enemy/Animation/JustGuard_Montage.JustGuard_Montage")
          (`KismetSystemLibrary.Delay` 5.0)
          (`self.PlayAnimMontage` "/Game/JUNWOO/enemy/Animation/JustGuard_Montage.JustGuard_Montage")
          (`KismetSystemLibrary.Delay` 5.0)
          (bind (_gimmickend_2 _isgroggy_2 _isbigattack_2) (`/Game/JUNWOO/components/BPC_enemy_statsystem.Gimmick` (`self.BPC_enemy_statsystem`) _currentpargauge))
          (`Widget.SetVisibility` (`WidgetComponent.GetUserWidgetObject` (`self.Enemy_Widget`)) "Hidden")
          (set `self.Gimmick End` _gimmickend_2)
          (set `self.IsGroggy` _isgroggy_2)
          (set `self.IsBigAttack` _isbigattack_2)
          (set `self.State` false)))
      (else
        (bind _isdead (`/Game/JUNWOO/components/BPC_enemy_statsystem.AfterGimmick` (`self.BPC_enemy_statsystem`) Damage))
        (set `self.Is Dead` _isdead)))))

(event `self.ReceiveTick`
  (params (DeltaSeconds :type "Float (single-precision)"))
  (bind _returnvalue (`self.K2_GetActorLocation`))
  (bind _returnvalue_2 (`self.K2_GetActorLocation` (`GameplayStatics.GetPlayerCharacter` 0)))
  (if (`self.GimmickState`)
    (set `self.direction` (`KismetMathLibrary.Normal` (- _returnvalue_2 _returnvalue)))
    (`self.K2_SetActorLocation` (+ (`self.K2_GetActorLocation`) (* (`self.speed`) (`self.direction`) (`GameplayStatics.GetWorldDeltaSeconds`))))
    (if (`self.IsTracing`)
      (`self.K2_SetActorRotation` (`KismetMathLibrary.MakeRotator` 0.0 0.0 (.yaw (`KismetMathLibrary.FindLookAtRotation` _returnvalue _returnvalue_2))))
      (if (`self.State`)
        (if (`self.Is Gimmick`)
          (`/Game/JUNWOO/enemy/ABP_Enemy_2.SetEnemyIsGimmick` (`self.As ABP Enemy 2`))
          (set `self.GimmickState` false)
          (`PrimitiveComponent.SetCollisionEnabled` (`self.tmp_detecter`) "NoCollision")
          (`Widget.SetVisibility` (`WidgetComponent.GetUserWidgetObject` (`self.Enemy_Widget`)) "Visible")
          (set `self.GimmickSwith` false)
          (set `self.GimmickSwitch2` true)
          (set `self.Is Gimmick` false))
        (elif (`self.Is Gimmick`)
          _
          (elif (`self.GimmickSwitch2`)
            (if (`self.Gimmick End`)
              (`self.PlayAnimMontage` "/Game/JUNWOO/enemy/Animation/groggy_Montage.groggy_Montage")
              (`/Game/JUNWOO/enemy/ABP_Enemy_2.SetEnemyIsGroggy` (`self.As ABP Enemy 2`))
              (set `self.GimmickSwitch2` false)
              (`KismetSystemLibrary.Delay` 7.13)
              (set `self.GimmickState` true)
              (else
                (`self.PlayAnimMontage` "/Game/JUNWOO/enemy/Animation/No_Root.No_Root")
                (`/Game/JUNWOO/enemy/ABP_Enemy_2.SetEnemyIsBigAttack` (`self.As ABP Enemy 2`))
                (set `self.GimmickSwitch2` false)
                (`KismetSystemLibrary.Delay` 2.0)
                (`GameplayStatics.ApplyDamage` (`GameplayStatics.GetPlayerCharacter` 0) 200.0 null self)
                (set `self.GimmickState` true)))
            (elif (`self.Is Dead`)
              (`/Game/JUNWOO/enemy/ABP_Enemy_2.SetEnemyIsDead` (`self.As ABP Enemy 2`))
              (set `self.GimmickState` false)
              (`PrimitiveComponent.SetCollisionEnabled` (`self.attack range`) "NoCollision")
              (`PrimitiveComponent.SetCollisionEnabled` (`self.tmp_detecter`) "NoCollision")
              (bind _returnvalue_3 (`|CreateWidget` "/Game/JUNWOO/UI/Success_Playing.Success_Playing_C"))
              (`UserWidget.AddToViewport` _returnvalue_3 0)
              (bind _foundwidgets (`WidgetBlueprintLibrary.GetAllWidgetsOfClass` "/Game/JUNWOO/UI/Base_widget.Base_widget_C" false))
              (`KismetSystemLibrary.K2_ClearAndInvalidateTimerHandle` (`/Game/JUNWOO/UI/Base_widget.handle` (`|GetArrayItem` _foundwidgets)))
              (`PrimitiveComponent.SetCollisionEnabled` (`self.CapsuleComponent`) "NoCollision")
              (`KismetSystemLibrary.Delay` 5.0)
              (`self.K2_DestroyActor`)
              (`KismetSystemLibrary.QuitGame` null "Quit")))))
      (elif (`self.State`)
        (if (`self.Is Gimmick`)
          (`/Game/JUNWOO/enemy/ABP_Enemy_2.SetEnemyIsGimmick` (`self.As ABP Enemy 2`))
          (set `self.GimmickState` false)
          (`PrimitiveComponent.SetCollisionEnabled` (`self.tmp_detecter`) "NoCollision")
          (`Widget.SetVisibility` (`WidgetComponent.GetUserWidgetObject` (`self.Enemy_Widget`)) "Visible")
          (set `self.GimmickSwith` false)
          (set `self.GimmickSwitch2` true)
          (set `self.Is Gimmick` false))
        (elif (`self.Is Gimmick`)
          _
          (elif (`self.GimmickSwitch2`)
            (if (`self.Gimmick End`)
              (`self.PlayAnimMontage` "/Game/JUNWOO/enemy/Animation/groggy_Montage.groggy_Montage")
              (`/Game/JUNWOO/enemy/ABP_Enemy_2.SetEnemyIsGroggy` (`self.As ABP Enemy 2`))
              (set `self.GimmickSwitch2` false)
              (`KismetSystemLibrary.Delay` 7.13)
              (set `self.GimmickState` true)
              (else
                (`self.PlayAnimMontage` "/Game/JUNWOO/enemy/Animation/No_Root.No_Root")
                (`/Game/JUNWOO/enemy/ABP_Enemy_2.SetEnemyIsBigAttack` (`self.As ABP Enemy 2`))
                (set `self.GimmickSwitch2` false)
                (`KismetSystemLibrary.Delay` 2.0)
                (`GameplayStatics.ApplyDamage` (`GameplayStatics.GetPlayerCharacter` 0) 200.0 null self)
                (set `self.GimmickState` true)))
            (elif (`self.Is Dead`)
              (`/Game/JUNWOO/enemy/ABP_Enemy_2.SetEnemyIsDead` (`self.As ABP Enemy 2`))
              (set `self.GimmickState` false)
              (`PrimitiveComponent.SetCollisionEnabled` (`self.attack range`) "NoCollision")
              (`PrimitiveComponent.SetCollisionEnabled` (`self.tmp_detecter`) "NoCollision")
              (bind _returnvalue_4 (`|CreateWidget` "/Game/JUNWOO/UI/Success_Playing.Success_Playing_C"))
              (`UserWidget.AddToViewport` _returnvalue_4 0)
              (bind _foundwidgets_2 (`WidgetBlueprintLibrary.GetAllWidgetsOfClass` "/Game/JUNWOO/UI/Base_widget.Base_widget_C" false))
              (`KismetSystemLibrary.K2_ClearAndInvalidateTimerHandle` (`/Game/JUNWOO/UI/Base_widget.handle` (`|GetArrayItem` _foundwidgets_2)))
              (`PrimitiveComponent.SetCollisionEnabled` (`self.CapsuleComponent`) "NoCollision")
              (`KismetSystemLibrary.Delay` 5.0)
              (`self.K2_DestroyActor`)
              (`KismetSystemLibrary.QuitGame` null "Quit"))))))
    (elif (`self.State`)
      (if (`self.Is Gimmick`)
        (`/Game/JUNWOO/enemy/ABP_Enemy_2.SetEnemyIsGimmick` (`self.As ABP Enemy 2`))
        (set `self.GimmickState` false)
        (`PrimitiveComponent.SetCollisionEnabled` (`self.tmp_detecter`) "NoCollision")
        (`Widget.SetVisibility` (`WidgetComponent.GetUserWidgetObject` (`self.Enemy_Widget`)) "Visible")
        (set `self.GimmickSwith` false)
        (set `self.GimmickSwitch2` true)
        (set `self.Is Gimmick` false))
      (elif (`self.Is Gimmick`)
        _
        (elif (`self.GimmickSwitch2`)
          (if (`self.Gimmick End`)
            (`self.PlayAnimMontage` "/Game/JUNWOO/enemy/Animation/groggy_Montage.groggy_Montage")
            (`/Game/JUNWOO/enemy/ABP_Enemy_2.SetEnemyIsGroggy` (`self.As ABP Enemy 2`))
            (set `self.GimmickSwitch2` false)
            (`KismetSystemLibrary.Delay` 7.13)
            (set `self.GimmickState` true)
            (else
              (`self.PlayAnimMontage` "/Game/JUNWOO/enemy/Animation/JumpAttack_Montage.JumpAttack_Montage")
              (`/Game/JUNWOO/enemy/ABP_Enemy_2.SetEnemyIsBigAttack` (`self.As ABP Enemy 2`))
              (set `self.GimmickSwitch2` false)
              (`KismetSystemLibrary.Delay` 2.0)
              (`GameplayStatics.ApplyDamage` (`GameplayStatics.GetPlayerCharacter` 0) 200.0 null self)
              (set `self.GimmickState` true)))
          (elif (`self.Is Dead`)
            (`/Game/JUNWOO/enemy/ABP_Enemy_2.SetEnemyIsDead` (`self.As ABP Enemy 2`))
            (set `self.GimmickState` false)
            (`PrimitiveComponent.SetCollisionEnabled` (`self.attack range`) "NoCollision")
            (`PrimitiveComponent.SetCollisionEnabled` (`self.tmp_detecter`) "NoCollision")
            (bind _returnvalue_5 (`|CreateWidget` "/Game/JUNWOO/UI/Success_Playing.Success_Playing_C"))
            (`UserWidget.AddToViewport` _returnvalue_5 0)
            (bind _foundwidgets_3 (`WidgetBlueprintLibrary.GetAllWidgetsOfClass` "/Game/JUNWOO/UI/Base_widget.Base_widget_C" false))
            (`KismetSystemLibrary.K2_ClearAndInvalidateTimerHandle` (`/Game/JUNWOO/UI/Base_widget.handle` (`|GetArrayItem` _foundwidgets_3)))
            (`PrimitiveComponent.SetCollisionEnabled` (`self.CapsuleComponent`) "NoCollision")
            (`KismetSystemLibrary.Delay` 5.0)
            (`self.K2_DestroyActor`)
            (`KismetSystemLibrary.QuitGame` null "Quit")))))))

(event `StartRightAttack`
  ; 오른쪽 공격
  (`PrimitiveComponent.SetCollisionEnabled` (`self.RightHand`) "QueryOnly"))

(event `StartLegAttack`
  ; 발차기 공격
  (`PrimitiveComponent.SetCollisionEnabled` (`self.RightLeg`) "QueryOnly"))

(event `StartLeftAttack`
  ; 왼쪽 공격
  (`PrimitiveComponent.SetCollisionEnabled` (`self.LeftHand`) "QueryOnly"))

(event `StopLegAttack`
  ; 발차기 공격
  (`PrimitiveComponent.SetCollisionEnabled` (`self.RightLeg`) "NoCollision"))

(event `StopRightAttack`
  ; 오른쪽 공격
  (`PrimitiveComponent.SetCollisionEnabled` (`self.RightHand`) "NoCollision"))

(event `StopLeftAttack`
  ; 왼쪽 공격
  (`PrimitiveComponent.SetCollisionEnabled` (`self.LeftHand`) "NoCollision"))

(event `self.RightLeg.OnComponentBeginOverlap`
  (params (OverlappedComponent :type "PrimitiveComponent Object Reference") (OtherActor :type "Actor Object Reference") (OtherComp :type "PrimitiveComponent Object Reference") (OtherBodyIndex :type Integer) (bFromSweep :type Boolean) (SweepResult :type "HitResult Structure (by ref)"))
  ; 발차기 공격
  (`/Engine/EditorBlueprintResources/StandardMacros.DoOnce` false :!label _label
    (:`Completed`
      (bind _asbp_top_down_character (cast `/Game/TopDown/Blueprints/BP_TopDownCharacter` OtherActor))
      (`GameplayStatics.ApplyDamage` _asbp_top_down_character 50.0 null self))))

(event `self.LeftHand.OnComponentBeginOverlap`
  (params (OverlappedComponent :type "PrimitiveComponent Object Reference") (OtherActor :type "Actor Object Reference") (OtherComp :type "PrimitiveComponent Object Reference") (OtherBodyIndex :type Integer) (bFromSweep :type Boolean) (SweepResult :type "HitResult Structure (by ref)"))
  ; 왼쪽 공격
  (`/Engine/EditorBlueprintResources/StandardMacros.DoOnce` false :!label _label_2
    (:`Completed`
      (bind _asbp_top_down_character (cast `/Game/TopDown/Blueprints/BP_TopDownCharacter` OtherActor))
      (`GameplayStatics.ApplyDamage` _asbp_top_down_character 50.0 null self))))

(event `self.RightHand.OnComponentBeginOverlap`
  (params (OverlappedComponent :type "PrimitiveComponent Object Reference") (OtherActor :type "Actor Object Reference") (OtherComp :type "PrimitiveComponent Object Reference") (OtherBodyIndex :type Integer) (bFromSweep :type Boolean) (SweepResult :type "HitResult Structure (by ref)"))
  ; 오른쪽 공격
  (`/Engine/EditorBlueprintResources/StandardMacros.DoOnce` false :!label _label_3
    (:`Completed`
      (bind _asbp_top_down_character (cast `/Game/TopDown/Blueprints/BP_TopDownCharacter` OtherActor))
      (`GameplayStatics.ApplyDamage` _asbp_top_down_character 50.0 null self))))

(event `ResetLeg`
  ; 발차기 공격
  (goto _label :!via `Reset`))

(event `ResetLeft`
  ; 왼쪽 공격
  (goto _label_2 :!via `Reset`))

(event `ResetRight`
  ; 오른쪽 공격
  (goto _label_3 :!via `Reset`))

(event `StartGuard`
  ; 저스트 가드
  (`PrimitiveComponent.SetCollisionEnabled` (`self.Guard_Range`) "QueryOnly"))

(event `GuardEffectOn`
  (bind _returnvalue (`GameplayStatics.SpawnEmitterAtLocation` "/Game/M5VFXVOL2/Particles/Fire_for_Dir/Fire_Dir_07.Fire_Dir_07" (`self.K2_GetActorLocation`) (struct) (1.0 1.0 1.0) false)))

(event `GuardEffectOff`
  (`ActorComponent.K2_DestroyComponent` (stale `GuardEffectOn` _returnvalue)))

(event `StopGuard`
  ; 저스트 가드
  (`PrimitiveComponent.SetCollisionEnabled` (`self.Guard_Range`) "NoCollision")
  (if (`self.IsGuard`)
    (`GameplayStatics.ApplyDamage` (`GameplayStatics.GetPlayerCharacter` 0) 50.0 null self)
    (`KismetSystemLibrary.PrintString` "\"가드 실패\"" true true (struct :`G` 0.66 :`B` 1.0 :`A` 1.0) 10.0)))

(event `self.Guard_Range.OnComponentBeginOverlap`
  (params (OverlappedComponent :type "PrimitiveComponent Object Reference") (OtherActor :type "Actor Object Reference") (OtherComp :type "PrimitiveComponent Object Reference") (OtherBodyIndex :type Integer) (bFromSweep :type Boolean) (SweepResult :type "HitResult Structure (by ref)"))
  ; 저스트 가드
  (set `self.IsGuard` false)
  (`KismetSystemLibrary.PrintString` "\"가드 성공\"")
  (`KismetSystemLibrary.Delay` 2.0)
  (set `self.IsGuard` true))

(event `JumpAttackEffect`
  (`GameplayStatics.SpawnEmitterAtLocation` "/Game/M5VFXVOL2/Particles/Explosion/Fire_Exp_03.Fire_Exp_03" (`self.K2_GetActorLocation`)))

(fn `UpdateHealthBar`
  (params (CurrentParGauge :type "Float (double-precision)") (MaxParGauge :type "Float (double-precision)"))
  (bind _asenemy_widget (cast `/Game/JUNWOO/UI/Enemy_Widget` (`WidgetComponent.GetUserWidgetObject` (`self.Enemy_Widget`))))
  (`ProgressBar.SetPercent` (`/Game/JUNWOO/UI/Enemy_Widget.ParalyzationBar` _asenemy_widget) (/ CurrentParGauge MaxParGauge)))

(fn `UserConstructionScript`)