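; Enemy stat component that tracks health and a paralyzation gauge for a gimmick-based fight, both filled to max on BeginPlay.
; DecreaseHealth flags the gimmick phase at a fixed health threshold, while DecreaseParalyzation drains the gauge and reports when it empties.
; Gimmick turns the gauge state into big-attack or groggy and gimmick-end outputs.
; AfterGimmick applies further damage and sets death at zero health.
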(event `self.ReceiveBeginPlay`
  (`self.initialize stats`)
  (`self.initiallize paralyzation`))

(fn `AfterGimmick`
  (params (DamagePoint :type "Float (double-precision)"))
  (returns (IsDead :type Boolean))
  (bind _output_get (set `self.current health` (- (`self.current health`) DamagePoint)))
  (if (<= _output_get 0.0)
    (set `self.current health` 0.0)
    (bind _output_get_2 (set `self.IsDead` true))
    (return _output_get_2)))

(fn `decrease health`
  (params (damagePoint :type "Float (double-precision)"))
  (returns (IsGimmick :type Boolean) (CurrentHealth :type "Float (double-precision)"))
  (bind _output_get (set `self.current health` (- (`self.current health`) damagePoint)))
  (if (<= _output_get 250.0)
    (bind _output_get_2 (set `self.IsGimmick` true))
    (return _output_get_2 _output_get)))

(fn `decrease paralyzation`
  (params (par_damage :type "Float (double-precision)"))
  (returns (CurrentParGauge :type "Float (double-precision)") (MaxParGauge :type "Float (double-precision)") (GimmickSwitch3 :type Boolean))
  (bind _max_par_gauge (`self.max_par_gauge`))
  (bind _output_get (set `self.current_par_gauge` (- (`self.current_par_gauge`) par_damage)))
  (if (<= _output_get 0.0)
    (return _output_get _max_par_gauge true)
    (else
      (return _output_get _max_par_gauge false))))

(fn `Gimmick`
  (params (CurrentParGauge :type "Float (double-precision)"))
  (returns (GimmickEnd :type Boolean) (IsGroggy :type Boolean) (IsBigAttack :type Boolean))
  (if (> CurrentParGauge 0.0)
    (return false false true)
    (else
      (set `self.current_par_gauge` 0.0)
      (return true true false))))

(fn `initialize stats`
  (set `self.current health` (`self.max health`)))

(fn `initiallize paralyzation`
  (set `self.current_par_gauge` (`self.max_par_gauge`)))